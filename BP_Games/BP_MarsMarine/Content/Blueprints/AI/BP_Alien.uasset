(event EventBeginPlay
  (if (not (Variables|Default|GetDead)) :!label _label
    (AI|AIMoveTo self "0, 0, 0" (Game|GetPlayerCharacter 0) 5.0 false
      (:OnSuccess
        _)
      (:OnFail
        _))
    (Utilities|FlowControl|Delay 0.1)
    (goto _label)))

(event Game|Damage|EventAnyDamage
  (params (Damage :type Float%20%28single-precision%29) (DamageType :type Damage%20Type%20Object%20Reference) (InstigatedBy :type Controller%20Object%20Reference) (DamageCauser :type Actor%20Object%20Reference))
  (if (not (Variables|Default|GetDead))
    (CallFunction|DecreaseHealth Damage)
    (CallFunction|KillAI)
    (Utilities|FlowControl|Delay 3.0)
    (Actor|DestroyActor)))

(event EventTick
  (params (DeltaSeconds :type Float%20%28single-precision%29))
  (if (not (Variables|Default|GetDead))
    (if (CallFunction|IsWithinAttackRange)
      (if (not (CallFunction|IsAttacking))
        (Components|Activation|Deactivate (Variables|Character|GetCharacterMovement))
        (Animation|Montage|PlayMontage (Variables|Character|GetMesh) "/Game/Blueprints/AI/AlienAttack1.AlienAttack1"
          (:then
            (Components|Activation|Activate (Variables|Character|GetCharacterMovement) false)))))))

(fn ConstructionScript)

(fn IsWithinAttackRange
  (return (< (Transformation|GetDistanceTo (Game|GetPlayerCharacter 0)) (Variables|Default|GetAttackRange))))

(fn IsAttacking
  (return (Animation|Montage|MontageIsPlaying (Components|SkeletalMesh|GetAnimInstance (Variables|Character|GetMesh)) "/Game/Blueprints/AI/AlienAttack1.AlienAttack1")))

(fn DamagePlayer
  (if (not (Variables|Default|GetDead))
    (Game|Damage|ApplyDamage (Game|GetPlayerCharacter 0) (Variables|Default|GetDamagePerHit) 0 0)))

(fn DecreaseHealth
  (params (B :type Float%20%28single-precision%29))
  (bind _output_get (Variables|Default|SetHealth (Math|Float|Clamp(Float) (- (Variables|Default|GetHealth) B) 0.0 1e+02)))
  (return _output_get))

(fn KillAI
  (bind _charactermovement (Variables|Character|GetCharacterMovement))
  (bind _output_get (Variables|Default|SetDead (== (Variables|Default|GetHealth) 0.0)))
  (if _output_get
    (Components|Movement|StopMovementImmediately _charactermovement)
    (Components|Activation|Deactivate _charactermovement)
    (Collision|SetActorEnableCollision false)
    (bind _asbp_marine (Utilities|Casting|CastToBP_Marine (Game|GetPlayerCharacter 0)))
    (Default|IncreaseKills _asbp_marine)
    (bind _asbp_mars_marine_game_mode (Utilities|Casting|CastToBP_MarsMarine_GameMode (Game|GetGameMode)))
    (Default|RegisterAlienDeath _asbp_mars_marine_game_mode self)))
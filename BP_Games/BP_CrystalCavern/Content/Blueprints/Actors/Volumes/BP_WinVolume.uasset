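; Level exit volume that completes the level when the player overlaps it with no BP_Crystal actors left in the world.
; If crystals remain, it prints how many are left instead.
; On completion it finds the current level's index in the LevelNames array and opens the next entry, or quits the game on the last one.
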(event Collision|EventActorBeginOverlap
  (params (OtherActor :type Actor%20Object%20Reference))
  (bind (_nocrystalsleft _numberofcrystals) (CallFunction|CrystalsRemain))
  (Utilities|IsPlayer OtherActor
    (:IsPlayer
      (if _nocrystalsleft
        (LevelMenagment|CompleteLevel)
        (else
          (Development|PrintString (Utilities|String|Append (Utilities|String|ToString(Integer) _numberofcrystals) " CRYSTALS LEFT")))))))

(fn ConstructionScript)

(fn CrystalsRemain
  (bind _outactors (Actor|GetAllActorsOfClass "/Game/Blueprints/Actors/Collectables/BP_Crystal.BP_Crystal_C"))
  (return (== (Utilities|Array|Length _outactors) 0) (Utilities|Array|Length _outactors)))

(fn CompleteLevel
  (if (LevelMenagment|IsThisLastLevel)
    (Game|QuitGame 0 "Quit" false)
    (else
      (LevelMenagment|LoadNextLevel))))

(fn GetCurrentLevelIndex
  (bind _returnvalue (Game|GetCurrentLevelName true))
  (return (Utilities|Array|FindItem (Variables|Default|GetLevelNames) (Utilities|String|StringToName _returnvalue))))

(fn IsThisLastLevel
  (return (== (LevelMenagment|GetCurrentLevelIndex) (Utilities|Array|LastIndex (Variables|Default|GetLevelNames)))))

(fn LoadNextLevel
  (Game|OpenLevel(byName) (LevelMenagment|GetNextLevelName)))

(fn GetNextLevelName
  (return (Utilities|Array|Get(acopy) (Variables|Default|GetLevelNames) (+ (LevelMenagment|GetCurrentLevelIndex) 1))))
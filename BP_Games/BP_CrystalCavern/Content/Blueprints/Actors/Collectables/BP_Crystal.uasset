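; BP_Crystal is a collectable crystal actor that the player picks up by overlapping it.
; On overlap it stores its location, scale and light intensity, then plays a collection timeline.
; Timeline curves lerp it toward the player pawn's current position while shrinking it to zero and fading CrystalLight.
; When the timeline finishes, the actor destroys itself.
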(event Collision|EventActorBeginOverlap
  (params (OtherActor :type Actor%20Object%20Reference))
  (Utilities|IsPlayer OtherActor
    (:IsPlayer
      (CallFunction|StoreStartingValues)
      (bind (_direction _collectionprogress _scaleprogress _lightintensity) (Timeline|CollectionTimeline Play)
        (:Update
          (CallFunction|MovetoPlayer _collectionprogress)
          (CallFunction|ScaleCrystal _scaleprogress)
          (CallFunction|LightIntensity _lightintensity))
        (:Finished
          (Actor|DestroyActor))))))

(fn ConstructionScript)

(fn MovetoPlayer
  (params (Alpha :type Float%20%28single-precision%29))
  (Transformation|SetActorLocation (Math|Vector|Lerp(Vector) (Variables|Default|GetStartLocation) (Transformation|GetActorLocation (Game|Player|GetPlayerPawn 0)) Alpha) false false))

(fn StoreStartingValues
  (Variables|Default|SetStartLocation (Transformation|GetActorLocation))
  (Variables|Default|SetStartScale (Transformation|GetActorScale3D))
  (Variables|Default|SetStartLightIntensity (Variables|/Script/Engine.LightComponentBase|GetIntensity (Variables|Default|GetCrystalLight))))

(fn ScaleCrystal
  (params (Alpha :type Float%20%28single-precision%29))
  (Transformation|SetActorScale3D (Math|Vector|Lerp(Vector) (Variables|Default|GetStartScale) "0, 0, 0" Alpha)))

(fn LightIntensity
  (params (Alpha :type Float%20%28single-precision%29))
  (Rendering|Components|Light|SetIntensity (Variables|Default|GetCrystalLight) (Math|Float|Lerp (Variables|Default|GetStartLightIntensity) 0.0 Alpha)))
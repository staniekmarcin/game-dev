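; BP_PlayerPawn is the player-controlled rolling ball pawn, which fades the camera in when play begins.
; Forward/Backward input applies acceleration-based torque to BallShape on both X and Y, while Right/Left input is unimplemented.
; Any damage calls CameraFade, which fades to black once and returns its duration for a delay before ReloadLevel reopens the current level.
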(event EventBeginPlay
  ;[1 1 1] BeginPlayCameraFade
  (CameraFades|StartCameraFade :self (Game|GetPlayerCameraManager 0) :FromAlpha 1.0 :Duration (Variables|Default|GetBaginPlayCameraFadeDuration,%20s) :bHoldWhenFinished true))

(event Game|Damage|EventAnyDamage
  (params (Damage :type Float%20%28single-precision%29) (DamageType :type Damage%20Type%20Object%20Reference) (InstigatedBy :type Controller%20Object%20Reference) (DamageCauser :type Actor%20Object%20Reference))
  (bind _camerafadeduration__s (CallFunction|CameraFade))
  (Utilities|FlowControl|Delay _camerafadeduration__s)
  (CallFunction|ReloadLevel))

(event Input|AxisEvents|InputAxisForward/Backward
  (params (AxisValue :type Float%20%28single-precision%29))
  (bind _ballrotationmultiply (Variables|Default|GetBallRotationMultiply))
  ;[1 1 1] RollingBall
  (Class|PrimitiveComponent|AddTorqueinRadians (Variables|Default|GetBallShape) (Math|Vector|MakeVector (* AxisValue _ballrotationmultiply) (* (stale Input|AxisEvents|InputAxisRight/Left AxisValue) _ballrotationmultiply) 0.0) "None" true))

(event Input|AxisEvents|InputAxisRight/Left
  (params (AxisValue :type Float%20%28single-precision%29))
  ;[1 1 1] RollingBall
)

(fn ConstructionScript)

(fn CameraFade
  (bind _camerafadeduration__s (Variables|Default|GetCameraFadeDuration,%20s))
  (Utilities|FlowControl|DoOnce false
    (:Completed
      (CameraFades|StartCameraFade (Game|GetPlayerCameraManager 0) 0.0 1.0 _camerafadeduration__s "(R=0.000000,G=0.000000,B=0.000000,A=1.000000)" false true)
      (return _camerafadeduration__s))))

(fn ReloadLevel
  (bind _returnvalue (Game|GetCurrentLevelName true))
  (Game|OpenLevel(byName) (Utilities|String|StringToName _returnvalue)))
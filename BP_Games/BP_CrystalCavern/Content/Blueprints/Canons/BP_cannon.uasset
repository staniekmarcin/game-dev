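; BP_cannon is a cannon that fires BP_Projectile actors repeatedly from the start of play.
; After a start delay it spawns a scaled projectile at ProjectileSpawnPoint, then plays the CannonFireRate timeline, which slides the cannon mesh along its relative X axis.
; The timeline's Cannon Fire event loops back to the delay, so StartShootingDelay precedes every shot and the timeline sets the rest of the cadence.
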(event EventBeginPlay
  (Utilities|FlowControl|Delay (Variables|CannonProperties|GetStartShootingDelay) :!label _label)
  (CallFunction|SpawnProjectile)
  (bind _cannonlocation (Timeline|CannonFireRate PlayFromStart)
    (:Update
      (CallFunction|MoveCannon _cannonlocation))
    (:CannonFire
      (goto _label))))

(fn ConstructionScript)

(fn SpawnProjectile
  (bind _projectilespawnpoint (Variables|Default|GetProjectileSpawnPoint))
  (Game|SpawnActorfromClass "/Game/Blueprints/Projectiles/BP_Projectile.BP_Projectile_C" (Math|Transform|MakeTransform (Transformation|GetWorldLocation _projectilespawnpoint) (Transformation|GetWorldRotation _projectilespawnpoint) (Math|Conversions|ToVector(Float) (Variables|CannonProperties|GetProjectileScale))) "Undefined" 0 0))

(fn MoveCannon
  (params (CannonYLocation :type Float%20%28single-precision%29))
  (Transformation|SetRelativeLocation (Variables|Default|GetCannon) (Math|Vector|MakeVector CannonYLocation 0.0 0.0) false false))
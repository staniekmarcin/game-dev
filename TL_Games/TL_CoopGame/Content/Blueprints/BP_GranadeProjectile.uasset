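; Grenade projectile actor that explodes on a timed fuse and then destroys itself.
; BeginPlay waits for ExplosionDelay before calling the Explode event, so detonation in this graph depends only on time, not impact.
; Explode spawns an explosion particle, applies radial damage credited to the instigator's controller and draws a debug sphere showing the damage radius.
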(event Custom|Explode
  (Effects|SpawnEmitteratLocation "/Game/WeaponEffects/Explosion/P_Explosion.P_Explosion" (Transformation|GetActorLocation))
  (Game|Damage|ApplyRadialDamage (Variables|Default|GetBaseDamage) (Transformation|GetActorLocation) (Variables|Default|GetDamageRadius) 0 0 self (Game|GetInstigatorController) false "ECC_Visibility")
  (Rendering|Debug|DrawDebugSphere (Transformation|GetActorLocation) (Variables|Default|GetDamageRadius) 12 "(R=1.000000,G=0.826640,B=0.024942,A=1.000000)" 2.0 1.0))

(event EventBeginPlay
  (Utilities|FlowControl|Delay (Variables|Default|GetExplosionDelay))
  (CallFunction|Explode)
  (Actor|DestroyActor))

(fn ConstructionScript)
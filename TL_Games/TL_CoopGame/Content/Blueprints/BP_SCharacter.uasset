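; BP_SCharacter is a character Blueprint that carries a grenade launcher and fires it on left mouse click.
; On BeginPlay it spawns BP_GranadeLauncher with itself as owner, stores it as CurrentWeapon and snaps it to the mesh's WeaponSocket.
; It also adds the WBP_CrossHair widget to the viewport.
; The mouse press calls Fire on CurrentWeapon, leaving the firing logic to the weapon.
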(event EventBeginPlay
  (bind _returnvalue (Game|SpawnActorfromClass "/Game/Blueprints/BP_granadeLauncher.BP_GranadeLauncher_C" (Math|Transform|MakeTransform "0, 0, 0") "AlwaysSpawn" self 0))
  (bind _output_get (Variables|Default|SetCurrentWeapon _returnvalue))
  (Transformation|AttachComponentToComponent _output_get (Variables|Character|GetMesh) "WeaponSocket" "SnapToTarget" "SnapToTarget" "SnapToTarget" true)
  (bind _returnvalue_2 (UserInterface|CreateWidget "/Game/UI/WBP_CrossHair.WBP_CrossHair_C"))
  (UserInterface|Viewport|AddtoViewport _returnvalue_2 0))

(event Input|MouseEvents|LeftMouseButton
  (params (Key :type Key%20Structure :default "None"))
  (:Pressed
    (Class|SWeapon|Fire (Variables|Default|GetCurrentWeapon))))

(fn ConstructionScript)